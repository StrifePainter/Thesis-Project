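; Playable character for a local two-player 2D fighting game, with side-to-side movement, jumping, blocking, ground and air attacks, and death.
; Player one's pawn takes Enhanced Input and key presses for both fighters, forwarding player two's actions to the second pawn, which is tinted when flagged.
; Attacks jump animation nodes and damage actors overlapping hit boxes.
; Blocking stops movement and reduces damage; death disables both pawns' input and calls the winner check.
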(event `Loadcontrols`
  (bind _asplayer_controller (cast `PlayerController` (`self.GetController`) :!label _label))
  (bind _returnvalue (pcsubsystem `EnhancedInputLocalPlayerSubsystem` _asplayer_controller))
  (`/Engine/EditorBlueprintResources/StandardMacros.IsValid` _returnvalue
    (:`Is Valid`
      (`EnhancedInputSubsystemInterface.AddMappingContext` _returnvalue "/Game/Controls/Fighting_IMC.Fighting_IMC" 0 (struct))
      (set `self.PlayerSpeed` (`CharacterMovementComponent.MaxWalkSpeed` (`self.CharacterMovement`)))
      (set `self.PlayerMaxHealth` (`self.Playerhealth`)))))

(event `self.ReceiveBeginPlay`
  (goto _label))

(event `AirAttack`
  ;[1 1 1] Handle Dealing Damage
  (for _array_element (`PrimitiveComponent.GetOverlappingActors` (`self.AirBox`) null)
    (if true
      (`GameplayStatics.ApplyDamage` _array_element (`self.Base Damage`)))))

(event `player2jump`
  ;[1 1 1] Handle Movement and Jumping
  (`self.Checkifblocking` :!label _label_2
    (:`else`
      _)
    (:`then`
      _))
  (`self.Jump`))

(event `EnhancedInput|/Game/Controls/Move_IA`
  (params (ActionValue :type "Float (double-precision)") (ElapsedSeconds :type "Float (double-precision)") (TriggeredSeconds :type "Float (double-precision)") (InputAction :type "InputAction Object Reference" :default "/Game/Controls/Move_IA.Move_IA"))
  ;[1 1 1] Handle Movement and Jumping
  (:`Triggered`
    (`self.AddMovementInput` (1.0 0.0 0.0) ActionValue)))

(event `EnhancedInput|/Game/Controls/Jump_IA`
  (params (ActionValue :type Boolean) (ElapsedSeconds :type "Float (double-precision)") (TriggeredSeconds :type "Float (double-precision)") (InputAction :type "InputAction Object Reference" :default "/Game/Controls/Jump_IA.Jump_IA"))
  ;[1 1 1] Handle Movement and Jumping
  (:`Started`
    (goto _label_2))
  (:`Completed`
    (`self.StopJumping`)))

(event `Blockplayer2`
  ;[1 1 1] Block System
  (if (not (`NavMovementComponent.IsFalling` (`self.CharacterMovement`))) :!label _label_3
    (set `self.Isblocking?` true)
    (set `CharacterMovementComponent.MaxWalkSpeed` 0.0 (`self.CharacterMovement`))))

(event `Attack`
  ;[1 1 1] Handle Dealing Damage
  (for _array_element (`PrimitiveComponent.GetOverlappingActors` (`self.AttackBox`) null)
    (if true
      (`GameplayStatics.ApplyDamage` _array_element (`self.Base Damage`)))))

(event `EnhancedInput|/Game/Controls/Block_IA`
  (params (ActionValue :type Boolean) (ElapsedSeconds :type "Float (double-precision)") (TriggeredSeconds :type "Float (double-precision)") (InputAction :type "InputAction Object Reference" :default "/Game/Controls/Block_IA.Block_IA"))
  ;[1 1 1] Block System
  (:`Started`
    (goto _label_3))
  (:`Completed`
    (set `self.Isblocking?` false :!label _label_4)
    (set `CharacterMovementComponent.MaxWalkSpeed` (`self.PlayerSpeed`) (`self.CharacterMovement`))))

(event `Stopblockingplayer2`
  ;[1 1 1] Block System
  (goto _label_4))

(event `Player2Attack`
  (`/Engine/EditorBlueprintResources/StandardMacros.DoOnce` false :!label _label_5
    (:`Completed`
      ;[1 1 1] Attack System
      (`self.Checkifblocking`
        (:`else`
          _)
        (:`then`
          _))
      ;;[1 1 1] Ground Attack
      (set `CharacterMovementComponent.MaxWalkSpeed` 0.0 (`self.CharacterMovement`))
      (if (`NavMovementComponent.IsFalling` (`self.CharacterMovement`))
        ;;[1 1 1] Air attack
        (`PaperZDAnimInstance.JumpToNode` (`PaperZDAnimationComponent.AnimInstance` (`self.AnimationComponent`)) "Airattack" "None")
        (`KismetSystemLibrary.Delay` (- (`PaperFlipbookComponent.GetFlipbookLength` (`self.Sprite`)) 0.5))
        (else
          (`PaperZDAnimInstance.JumpToNode` (`PaperZDAnimationComponent.AnimInstance` (`self.AnimationComponent`)) "Attack" "None")
          (`KismetSystemLibrary.Delay` (- (`PaperFlipbookComponent.GetFlipbookLength` (`self.Sprite`)) 0.5))))
      (set `CharacterMovementComponent.MaxWalkSpeed` (`self.PlayerSpeed`) (`self.CharacterMovement`))
      (goto _label_5 :!via `Reset`))))

(event `EnhancedInput|/Game/Controls/Attack_IA`
  (params (ActionValue :type Boolean) (ElapsedSeconds :type "Float (double-precision)") (TriggeredSeconds :type "Float (double-precision)") (InputAction :type "InputAction Object Reference" :default "/Game/Controls/Attack_IA.Attack_IA"))
  (:`Started`
    (goto _label_5)))

(event `self.ReceiveAnyDamage`
  (params (Damage :type "Float (single-precision)") (DamageType :type "DamageType Object Reference") (InstigatedBy :type "Controller Object Reference") (DamageCauser :type "Actor Object Reference"))
  ;[1 1 1] Handle Taken Damage
  (bind _output_get (set `self.Playerhealth` (select `bool` (`self.Isblocking?`) :`false` (- (`self.Playerhealth`) Damage) :`true` (- (`self.Playerhealth`) (/ Damage 5.0)))))
  (`self.Updatehealth`)
  (if (<= _output_get 0.0)
    (`/Engine/EditorBlueprintResources/StandardMacros.DoOnce` false
      (:`Completed`
        (`PaperZDAnimInstance.JumpToNode` (`PaperZDAnimationComponent.AnimInstance` (`self.AnimationComponent`)) "Death" "None")
        (`self.DisableInput` (`GameplayStatics.GetPlayerPawn` 0) null)
        (`self.DisableInput` (`GameplayStatics.GetPlayerPawn` 1) null)
        (`self.Whowon`)))
    (elif (not (`self.Isblocking?`))
      (`PaperZDAnimInstance.JumpToNode` (`PaperZDAnimationComponent.AnimInstance` (`self.AnimationComponent`)) "Damaged" "None")
      (set `CharacterMovementComponent.MaxWalkSpeed` 0.0 (`self.CharacterMovement`))
      (`KismetSystemLibrary.RetriggerableDelay` (`PaperFlipbookComponent.GetFlipbookLength` (`self.Sprite`)))
      (if (not (`self.Isblocking?`))
        (set `CharacterMovementComponent.MaxWalkSpeed` (`self.PlayerSpeed`) (`self.CharacterMovement`))))))

(event `Moveplayer2`
  (params (axisvalue :type "Float (double-precision)"))
  ;[1 1 1] Move player 2
  (`self.AddMovementInput` (1.0 0.0 0.0) axisvalue))

(event `EnhancedInput|/Game/Controls/MovePlayer2_AI`
  (params (ActionValue :type "Float (double-precision)") (ElapsedSeconds :type "Float (double-precision)") (TriggeredSeconds :type "Float (double-precision)") (InputAction :type "InputAction Object Reference" :default "/Game/Controls/MovePlayer2_AI.MovePlayer2_AI"))
  (bind _player2 (`self.player2`))
  ;[1 1 1] Move player 2
  (:`Triggered`
    (`/Engine/EditorBlueprintResources/StandardMacros.IsValid` _player2
      (:`Is Valid`
        (`self.Moveplayer2` _player2 ActionValue))
      (:`Is Not Valid`
        (bind _asplayercharacterbp (cast `/Game/Blueprints/playercharacterbp` (`GameplayStatics.GetPlayerPawn` 1)))
        (bind _output_get (set `self.player2` _asplayercharacterbp))
        (`self.Moveplayer2` _output_get ActionValue)))))

(event `Key|Up`
  (params (Key :type "Key Structure"))
  (bind _player2 (`self.player2`))
  ;[1 1 1] Move player 2
  (:`Pressed`
    (`/Engine/EditorBlueprintResources/StandardMacros.IsValid` _player2
      (:`Is Valid`
        (`self.player2jump` _player2))
      (:`Is Not Valid`
        (bind _asplayercharacterbp (cast `/Game/Blueprints/playercharacterbp` (`GameplayStatics.GetPlayerPawn` 1)))
        (bind _output_get (set `self.player2` _asplayercharacterbp))
        (`self.player2jump` _output_get)))))

(event `Key|Down`
  (params (Key :type "Key Structure"))
  (bind _player2 (`self.player2`))
  ;[1 1 1] Move player 2
  (:`Pressed`
    (`/Engine/EditorBlueprintResources/StandardMacros.IsValid` _player2
      (:`Is Valid`
        (`self.Player2Attack` _player2))
      (:`Is Not Valid`
        (bind _asplayercharacterbp (cast `/Game/Blueprints/playercharacterbp` (`GameplayStatics.GetPlayerPawn` 1)))
        (bind _output_get (set `self.player2` _asplayercharacterbp))
        (`self.Player2Attack` _output_get)))))

(event `EnhancedInput|/Game/Controls/BlockPlayer2_IA`
  (params (ActionValue :type Boolean) (ElapsedSeconds :type "Float (double-precision)") (TriggeredSeconds :type "Float (double-precision)") (InputAction :type "InputAction Object Reference" :default "/Game/Controls/BlockPlayer2_IA.BlockPlayer2_IA"))
  ;[1 1 1] Move player 2
  (:`Started`
    (`/Engine/EditorBlueprintResources/StandardMacros.IsValid` (`self.player2`)
      (:`Is Valid`
        (`self.Blockplayer2` (`self.player2`)))
      (:`Is Not Valid`
        (bind _asplayercharacterbp (cast `/Game/Blueprints/playercharacterbp` (`GameplayStatics.GetPlayerPawn` 1)))
        (set `self.player2` _asplayercharacterbp)
        (`self.Blockplayer2`))))
  (:`Completed`
    (`/Engine/EditorBlueprintResources/StandardMacros.IsValid` (`self.player2`)
      (:`Is Valid`
        (`self.Stopblockingplayer2` (`self.player2`)))
      (:`Is Not Valid`
        (bind _asplayercharacterbp_2 (cast `/Game/Blueprints/playercharacterbp` (`GameplayStatics.GetPlayerPawn` 1)))
        (set `self.player2` _asplayercharacterbp_2)
        (`self.Stopblockingplayer2`)))))

(fn `UserConstructionScript`
  (if (`self.isplayer2?`)
    (`PaperFlipbookComponent.SetSpriteColor` (`self.Sprite`) (struct :`R` 1.0 :`G` 0.643667 :`B` 0.125 :`A` 1.0))))